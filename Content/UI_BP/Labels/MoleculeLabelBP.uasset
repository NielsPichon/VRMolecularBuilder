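; MoleculeLabelBP is a world-space label actor that displays a molecule name through a widget component.
; Each tick it rotates its Scene component to face the motion controller pawn's camera, billboard style.
; SetText passes the given text to the MoleculeName widget, replacing periods with colons.
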(event EventTick
  (params (DeltaSeconds :type Float%20%28single-precision%29))
  (bind _asmotion_controller_pawn (Utilities|Casting|CastToMotionControllerPawn (Game|Player|GetPlayerPawn 0)))
  (Transformation|SetWorldRotation (Variables|Default|GetScene) (Math|Rotator|MakeRotator (.roll (Math|Rotator|FindLookatRotation (Transformation|GetWorldLocation (Variables|Default|GetDefaultSceneRoot)) (Transformation|GetWorldLocation (Variables|/Game/VirtualRealityBP/Blueprints/MotionControllerPawn.MotionControllerPawn_C|GetCamera _asmotion_controller_pawn)))) (.pitch (Math|Rotator|FindLookatRotation (Transformation|GetWorldLocation (Variables|Default|GetDefaultSceneRoot)) (Transformation|GetWorldLocation (Variables|/Game/VirtualRealityBP/Blueprints/MotionControllerPawn.MotionControllerPawn_C|GetCamera _asmotion_controller_pawn)))) (.yaw (Math|Rotator|FindLookatRotation (Transformation|GetWorldLocation (Variables|Default|GetDefaultSceneRoot)) (Transformation|GetWorldLocation (Variables|/Game/VirtualRealityBP/Blueprints/MotionControllerPawn.MotionControllerPawn_C|GetCamera _asmotion_controller_pawn))))) false false))

(fn ConstructionScript)

(fn SetText
  (params (Text :type String))
  (bind _asmolecule_name (Utilities|Casting|CastToMoleculeName (UserInterface|GetUserWidgetObject (Variables|Default|GetWidget))))
  (Default|SetText _asmolecule_name (Utilities|String|Replace Text "." ": ")))