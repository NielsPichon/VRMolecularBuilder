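; GrabMoleculeBP is an actor, filed among the UI labels, that turns to face the player's camera on the motion controller pawn.
; Each Tick it casts player pawn 0 to MotionControllerPawn and finds the look-at rotation toward that camera.
; It eases toward that rotation with RInterpTo and applies only the yaw, so it stays upright.
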(event EventTick
  (params (DeltaSeconds :type Float%20%28single-precision%29))
  (bind _asmotion_controller_pawn (Utilities|Casting|CastToMotionControllerPawn (Game|Player|GetPlayerPawn 0)))
  (Transformation|SetActorRotation (Math|Rotator|MakeRotator 0.0 0.0 (.Yaw (Math|Rotator|BreakRotator (Math|Interpolation|RInterpTo (Transformation|GetActorRotation) (Math|Rotator|FindLookatRotation (Transformation|GetActorLocation) (Transformation|GetWorldLocation (Variables|/Game/VirtualRealityBP/Blueprints/MotionControllerPawn.MotionControllerPawn_C|GetCamera _asmotion_controller_pawn))) (Utilities|Time|GetWorldDeltaSeconds) 5.0))))))

(fn ConstructionScript)