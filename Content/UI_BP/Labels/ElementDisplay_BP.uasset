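; ElementDisplay_BP is a world-space label actor that shows an element text through an ElementDisplay widget component.
; SetText passes the given text to the widget's SetElement function.
; Each tick, it turns the widget in yaw only to face the camera of the player's MotionControllerPawn, so the label stays upright and readable in VR.
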(event EventTick
  (params (DeltaSeconds :type Float%20%28single-precision%29))
  (bind _asmotion_controller_pawn (Utilities|Casting|CastToMotionControllerPawn (Game|Player|GetPlayerPawn 0)))
  (Transformation|SetWorldRotation (Variables|Default|GetWidget) (Math|Rotator|MakeRotator 0.0 0.0 (.yaw (Math|Rotator|FindLookatRotation (Transformation|GetWorldLocation (Variables|Default|GetDefaultSceneRoot)) (Transformation|GetWorldLocation (Variables|/Game/VirtualRealityBP/Blueprints/MotionControllerPawn.MotionControllerPawn_C|GetCamera _asmotion_controller_pawn))))) false false))

(fn ConstructionScript)

(fn SetText
  (params (Text :type String))
  (bind _aselement_display (Utilities|Casting|CastToElementDisplay (UserInterface|GetUserWidgetObject (Variables|Default|GetWidget))))
  (Default|SetElement _aselement_display Text))