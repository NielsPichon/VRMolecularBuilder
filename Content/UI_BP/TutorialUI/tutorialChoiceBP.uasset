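; Tutorial choice actor that presents two computer-button child actors and reports a yes/no answer.
; On BeginPlay it binds both UI_ComputerBttn children's click events to a single handler.
; The handler broadcasts ChoiceMade, true when the clicked button's letter is "YES", then destroys both buttons and itself, making it a one-shot prompt.
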(event Custom|BttnClicked
  (params (Destination :type BttnTarget%20Enum :default "NewEnumerator0") (Letter :type String))
  (Default|CallChoiceMade (Utilities|Enum|Equal(Enum) Letter "YES"))
  (Actor|DestroyActor (Variables|/Script/Engine.ChildActorComponent|GetChildActor (Variables|Default|GetUI_ComputerBttn)))
  (Actor|DestroyActor (Variables|/Script/Engine.ChildActorComponent|GetChildActor (Variables|Default|GetChildActor)))
  (Actor|DestroyActor))

(event EventBeginPlay
  (bind _asui_computer_bttn (Utilities|Casting|CastToUI_ComputerBttn (Variables|/Script/Engine.ChildActorComponent|GetChildActor (Variables|Default|GetChildActor))))
  (EventDispatchers|BindEventtoBttnIsClicked _asui_computer_bttn (delegate Custom|BttnClicked))
  (bind _asui_computer_bttn_2 (Utilities|Casting|CastToUI_ComputerBttn (Variables|/Script/Engine.ChildActorComponent|GetChildActor (Variables|Default|GetUI_ComputerBttn))))
  (EventDispatchers|BindEventtoBttnIsClicked _asui_computer_bttn_2 (delegate Custom|BttnClicked)))

(fn ConstructionScript)